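; BP_PeopleManager polls people-counting sensors over UDP and shows their counts as on-screen debug text.
; On BeginPlay it starts a JSON receiver and a looping timer that sends a capture command through the UDP sender.
; Each received packet is parsed into a sensor map, printing counts for three hardcoded sensor IDs.
; SENSORE001 prints without a presence check, and SENSORE003 is only checked when SENSORE002 is present.
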(event OnJsonReceived(UDPJsonReceiver)
  (params (JsonString :type String))
  ;[1 1 1] Sistema di ricezione e del conto delle persone dalla mappa dei sensori presenti
  (bind _outsensors (Class|PeopleCounterJsonLib|ParsePeopleCountPacket JsonString))
  (Development|PrintString (Utilities|String|Append (Utilities|String|ToString(Integer) (.Value (Utilities|Map|Find _outsensors "SENSORE001"))) "PERSONE (SENSORE001)"))
  (if (.ReturnValue (Utilities|Map|Find _outsensors "SENSORE002"))
    (Development|PrintString (Utilities|String|Append (Utilities|String|ToString(Integer) (.Value (Utilities|Map|Find _outsensors "SENSORE002"))) "PERSONE (SENSORE002)") true true "(R=0.000000,G=1.000000,B=0.097294,A=1.000000)")
    (if (.ReturnValue (Utilities|Map|Find _outsensors "SENSORE003"))
      (Development|PrintString (Utilities|String|Append (Utilities|String|ToString(Integer) (.Value (Utilities|Map|Find _outsensors "SENSORE003"))) "PERSONE (SENSORE002)") true true "(R=1.000000,G=0.051108,B=0.000000,A=1.000000)")
      (else
        (Development|PrintString "“SENSORE003 non nel pacchetto (0/offline)”" true true "(R=1.000000,G=0.000000,B=0.075452,A=1.000000)")))
    (else
      (Development|PrintString "“SENSORE002 non nel pacchetto (0/offline)”" true true "(R=0.083613,G=1.000000,B=0.000000,A=1.000000)"))))

(event Custom|Timer_CaptureStick
  ;[1 1 1] Sender e Reciever che con il timer ti permette di mandare il comando di cattura a tutti i tuoi sensori
  (Class|UDPJsonSenderComponent|SendJsonString (Variables|Default|GetUDPJsonSender) "{\"cmd\":\"capture\"}"))

(event EventBeginPlay
  ;[1 1 1] Sender e Reciever che con il timer ti permette di mandare il comando di cattura a tutti i tuoi sensori
  (Class|UDPJsonReceiverComponent|StartReceiver (Variables|Default|GetUDPJsonReceiver))
  (Utilities|Time|SetTimerbyEvent (delegate Custom|Timer_CaptureStick) 2.0 true))

(event Collision|EventActorBeginOverlap
  (params (OtherActor :type Actor%20Object%20Reference)))

(event EventTick
  (params (DeltaSeconds :type Float%20%28single-precision%29)))

(fn ConstructionScript)